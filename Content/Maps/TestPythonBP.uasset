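; TestPythonBP is a test Actor Blueprint whose functions, judging by its name and printed message, exist to exercise Blueprint access from Python.
; TestMethod prints a message and returns a string, while TestAdvancedMethod prints its mixed arguments and array input, returning two of the arguments from inside the loop.
; RuntimeSpawn spawns another instance of the same class at the origin, scaled up.
; The event graph and construction script contain no logic.
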(fn `RuntimeSpawn`
  (`|SpawnActorFromClass` "TestPythonBP_C" (`KismetMathLibrary.MakeTransform` (0.0 0.0 0.0) (struct) (20.0 20.0 20.0)) "Undefined" "MultiplyWithRoot" null null))

(fn `TestAdvancedMethod`
  (params (arg1 :type Boolean) (arg2 :type Integer) (arg3 :type String) (arg4 :type "Array of String"))
  (returns (out_arg1 :type Integer) (out_arg2 :type String))
  (`KismetSystemLibrary.PrintString` (`KismetStringLibrary.Concat_StrStr` (`KismetStringLibrary.Conv_BoolToString` arg1) "|||" (`KismetStringLibrary.Conv_IntToString` arg2) "|||" arg3))
  (for _array_element arg4
    (`KismetSystemLibrary.PrintString` _array_element)
    (return arg2 arg3)))

(fn `TestMethod`
  (returns (Ret :type String))
  (`KismetSystemLibrary.PrintString` "This is a bp test for python!")
  (return "test"))

(fn `UserConstructionScript`)